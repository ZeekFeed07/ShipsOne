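; BP_ShGameplayPawn is the player camera pawn for ShipsOne, with events to rotate, move and zoom a spring arm camera.
; Rotation feeds yaw to the controller and sets spring arm pitch within a clamped angle range.
; Movement drives a FloatingPawnMovement along the arm's flattened forward and right vectors, so panning stays horizontal and follows the view.
; Zoom adjusts the arm length within fixed limits.
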(event EventMoveCamera2D
  (params (Angle :type Vector%202D%20Structure%20%28by%20ref%29))
  (bind _springarm (Variables|Default|GetSpringArm))
  (bind _returnvalue (Math|Vector|GetForwardVector _springarm))
  (bind _returnvalue_2 (* _returnvalue (.y Angle)))
  (Class|PawnMovementComponent|AddInputVector (Variables|Default|GetFloatingPawnMovement) (+ (Math|Vector|Normalize (Math|Vector|MakeVector (.x _returnvalue_2) (.y _returnvalue_2) 0.0)) (* (.x Angle) (Math|Vector|GetRightVector (Variables|Default|GetSpringArm)))) false))

(event EventZoomCamera
  (params (Value :type Float%20%28single-precision%29))
  (Variables|/Script/Engine.SpringArmComponent|SetTargetArmLength (Variables|Default|GetSpringArm) (Math|Float|Clamp(Float) (+ (* Value 5e+01) (Variables|/Script/Engine.SpringArmComponent|GetTargetArmLength (Variables|Default|GetSpringArm))) 1e+03 2e+03)))

(event EventRotateCameraAngle2D
  (params (Angle :type Vector%202D%20Structure%20%28by%20ref%29))
  (bind _springarm (Variables|Default|GetSpringArm))
  (bind _relativerotation (Variables|/Script/Engine.SceneComponent|GetRelativeRotation _springarm))
  (Pawn|Input|AddControllerYawInput (.x Angle))
  (Transformation|SetRelativeRotation (Variables|Default|GetSpringArm) (Math|Rotator|MakeRotator (.roll _relativerotation) (Math|Float|ClampAngle (+ (* (.y Angle) 2.0) (.pitch _relativerotation)) 2.8e+02 3.4e+02) (.yaw _relativerotation)) false false))

(fn ConstructionScript)