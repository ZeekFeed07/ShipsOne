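; Player camera pawn for the ship game, handling rotate, move and zoom on a spring arm, with camera settings read from PawnConfig on BeginPlay.
; When the controller replicates, it casts to ShGameplayPlayerController and binds handlers to that controller's input events.
; Yaw and movement act on the actor, while pitch and unclamped zoom act on the spring arm.
; Place, rotate and pull ship handlers are bound but empty.
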(event EventBeginPlay
  (Utilities|FlowControl|Sequence
    (:then_0
      (bind _pawnconfig (Variables|Default|GetPawnConfig)
        (:then
          (Variables|Default|SetCameraDistance (Variables|/Script/ShipsOne.PawnDataAsset|GetCameraDistance _pawnconfig))
          (Variables|Default|SetCameraMovementSpeed (Variables|/Script/ShipsOne.PawnDataAsset|GetCameraMovementSpeed _pawnconfig))
          (Variables|Default|SetCameraRotationSpeed (Variables|/Script/ShipsOne.PawnDataAsset|GetCameraRotationSpeed _pawnconfig)))
        (:else)))
    (:then_1
      (Variables|/Script/Engine.SpringArmComponent|SetTargetArmLength (Variables|Default|GetSpringArmComponent) (Variables|Default|GetCameraDistance)))))

(event EventOnControllerReplicated
  (bind _assh_gameplay_player_controller (Utilities|Casting|CastToShGameplayPlayerController (Pawn|GetController))
    (:then
      (Variables|Default|SetControllerRefCasted _assh_gameplay_player_controller)
      (CallFunction|BindControllerInputs))
    (:CastFailed
      (Development|PrintString "Error: Player controller cast failed in BP_Pawn"))))

(event Custom|OnCameraRotationRecieved
  (params (Value :type Vector%202D%20Structure))
  (Class|Actor|AddActorWorldRotation (Math|Rotator|MakeRotator 0.0 0.0 (* (Variables|Default|GetCameraRotationSpeed) (.x Value))))
  (Transformation|AddRelativeRotation (Variables|Default|GetSpringArmComponent) (Math|Rotator|MakeRotator 0.0 (* (Variables|Default|GetCameraRotationSpeed) (.y Value)) 0.0) false false))

(event Custom|OnCameraMovementRecieved
  (params (Value :type Vector%202D%20Structure))
  (bind (_x _y) (Math|Vector2D|BreakVector2D Value))
  (bind _cameramovementspeed (Variables|Default|GetCameraMovementSpeed))
  (Transformation|AddActorLocalOffset (Math|Vector|MakeVector (* _x _cameramovementspeed) (* _y _cameramovementspeed) 0.0) false false))

(event Custom|OnCameraZoomRecieved
  (params (Value :type Float%20%28single-precision%29))
  (Variables|/Script/Engine.SpringArmComponent|SetTargetArmLength (Variables|Default|GetSpringArmComponent) (+ (* Value 1e+02) (Variables|/Script/Engine.SpringArmComponent|GetTargetArmLength (Variables|Default|GetSpringArmComponent)))))

(event Custom|OnPlaceShipRecieved
  (params (Value :type Boolean)))

(event Custom|OnRotateShipRecieved
  (params (Value :type Float%20%28single-precision%29)))

(event Custom|OnPullShipRecieved
  (params (Value :type Boolean)))

(fn ConstructionScript)

(fn BindControllerInputs
  (Variables|Default|GetControllerRefCasted
    (:then
      (Utilities|FlowControl|Sequence
        (:then_0
          (EventDispatchers|BindEventtoOnCameraRotationInput (Variables|Default|GetControllerRefCasted) (EventDispatchers|CreateEvent :!event Custom|OnCameraRotationRecieved)))
        (:then_1
          (EventDispatchers|BindEventtoOnCameraMovementInput (Variables|Default|GetControllerRefCasted) (EventDispatchers|CreateEvent :!event Custom|OnCameraMovementRecieved)))
        (:then_2
          (EventDispatchers|BindEventtoOnCameraZoomInput (Variables|Default|GetControllerRefCasted) (EventDispatchers|CreateEvent :!event Custom|OnCameraZoomRecieved)))
        (:then_3
          (EventDispatchers|BindEventtoOnPlaceShipInput (Variables|Default|GetControllerRefCasted) (EventDispatchers|CreateEvent :!event Custom|OnPlaceShipRecieved)))
        (:then_4
          (EventDispatchers|BindEventtoOnRotateShipInput (Variables|Default|GetControllerRefCasted) (EventDispatchers|CreateEvent :!event Custom|OnRotateShipRecieved)))
        (:then_5
          (EventDispatchers|BindEventtoOnPullShipInput (Variables|Default|GetControllerRefCasted) (EventDispatchers|CreateEvent :!event Custom|OnPullShipRecieved)))))
    (:else
      (Development|PrintString "Error: Player controller not valid in BP_Pawn"))))